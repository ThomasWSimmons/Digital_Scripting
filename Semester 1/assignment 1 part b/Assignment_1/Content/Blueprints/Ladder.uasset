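; Ladder Blueprint that lets the 2D side-scroller character climb while inside its collision box.
; On begin overlap it casts to 2DSideScrollerCharacter, sets IsInLadder, switches movement to Flying and zeroes gravity scale.
; On end overlap it clears the flag, returns movement to Walking and sets gravity scale back to a hardcoded value rather than a cached original.
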(event OnComponentBeginOverlap(Box)
  (params (OverlappedComponent :type Primitive%20Component%20Object%20Reference) (OtherActor :type Actor%20Object%20Reference) (OtherComp :type Primitive%20Component%20Object%20Reference) (OtherBodyIndex :type Integer) (bFromSweep :type Boolean) (SweepResult :type Hit%20Result%20Structure%20%28by%20ref%29))
  ;[0.5349 0.5662 1] 2D Player Entering Ladder
  (bind _as2dside_scroller_character (Utilities|Casting|CastTo2DSideScrollerCharacter OtherActor)) ; 2D Character has been found
  (Variables|/Game/2DSideScrollerBP/Blueprints/2DSideScrollerCharacter.2DSideScrollerCharacter_C|SetisInLadder _as2dside_scroller_character true) ; record player entering ladder
  (Pawn|Components|CharacterMovement|SetMovementMode (Variables|/Script/Engine.Character|GetCharacterMovement _as2dside_scroller_character) "MOVE_Flying" 0) ; change the player movement upwards
  (Variables|/Script/Engine.CharacterMovementComponent|SetGravityScale (Variables|/Script/Engine.Character|GetCharacterMovement _as2dside_scroller_character) 0.0) ; switch off gravity
)

(event OnComponentEndOverlap(Box)
  (params (OverlappedComponent :type Primitive%20Component%20Object%20Reference) (OtherActor :type Actor%20Object%20Reference) (OtherComp :type Primitive%20Component%20Object%20Reference) (OtherBodyIndex :type Integer))
  ;[0.4475 0.5927 1] 2D Player Exits Ladder
  (bind _as2dside_scroller_character (Utilities|Casting|CastTo2DSideScrollerCharacter OtherActor)) ; 2D Character has been found
  (Variables|/Game/2DSideScrollerBP/Blueprints/2DSideScrollerCharacter.2DSideScrollerCharacter_C|SetisInLadder _as2dside_scroller_character false) ; Record player entering the ladder
  (Pawn|Components|CharacterMovement|SetMovementMode (Variables|/Script/Engine.Character|GetCharacterMovement _as2dside_scroller_character) "MOVE_Walking" 0) ; change character movement to walking
  (Variables|/Script/Engine.CharacterMovementComponent|SetGravityScale (Variables|/Script/Engine.Character|GetCharacterMovement _as2dside_scroller_character) 2.0) ; reset gravity back to original state
)

(fn ConstructionScript)