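; A moving health platform for the 2D side scroller that heals the player character on contact.
; A timeline started on BeginPlay offsets the actor from the initial location cached in the construction script.
; Overlapping the Box casts to 2DSideScrollerCharacter and, after a short delay, adds a fixed amount to its Health.
; The heal has no clamp or check that the player is still overlapping, and the actor remains afterwards.
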(event OnComponentBeginOverlap(Box)
  (params (OverlappedComponent :type Primitive%20Component%20Object%20Reference) (OtherActor :type Actor%20Object%20Reference) (OtherComp :type Primitive%20Component%20Object%20Reference) (OtherBodyIndex :type Integer) (bFromSweep :type Boolean) (SweepResult :type Hit%20Result%20Structure%20%28by%20ref%29))
  (bind _as2dside_scroller_character (Utilities|Casting|CastTo2DSideScrollerCharacter (stale Custom|OnComponentBeginOverlap_Event_0 OtherActor))) ; Declaring 2D character
  (Utilities|FlowControl|Delay 1.0) ; Time delay before health is added on
  (Variables|/Game/2DSideScrollerBP/Blueprints/2DSideScrollerCharacter.2DSideScrollerCharacter_C|SetHealth _as2dside_scroller_character (+ (Variables|/Game/2DSideScrollerBP/Blueprints/2DSideScrollerCharacter.2DSideScrollerCharacter_C|GetHealth _as2dside_scroller_character) 0.14)) ; Declaring the new value of health for 2d character
)

(event Custom|OnComponentBeginOverlap_Event_0
  (params (OverlappedComponent :type Primitive%20Component%20Object%20Reference) (OtherActor :type Actor%20Object%20Reference) (OtherComp :type Primitive%20Component%20Object%20Reference) (OtherBodyIndex :type Integer) (bFromSweep :type Boolean) (SweepResult :type Hit%20Result%20Structure%20%28by%20ref%29))
  (bind _as2dside_scroller_character (Utilities|Casting|CastTo2DSideScrollerCharacter OtherActor)) ; Declaring 2D character
  (Utilities|FlowControl|Delay 1.0) ; Time delay before health is added on
  (Variables|/Game/2DSideScrollerBP/Blueprints/2DSideScrollerCharacter.2DSideScrollerCharacter_C|SetHealth _as2dside_scroller_character (+ (Variables|/Game/2DSideScrollerBP/Blueprints/2DSideScrollerCharacter.2DSideScrollerCharacter_C|GetHealth _as2dside_scroller_character) 0.14)) ; Declaring the new value of health for 2d character
)

(event EventBeginPlay
  (bind _newtrack_0 (Timeline|Health_Height_Left_Right Play) ; timeline of platform movement
    (:Update
      (Transformation|SetActorLocation (+ (Variables|Default|GetInitial%20Loaction) _newtrack_0) false false) ; declaring new platform location
    )))

(fn ConstructionScript
  (bind _returnvalue (Transformation|GetActorLocation))
  (Transformation|SetActorLocation _returnvalue false false)
  (Variables|Default|SetInitial%20Loaction _returnvalue))