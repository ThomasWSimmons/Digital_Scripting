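; Completion gate actor that moves along a timeline-driven path, presumably left and right, and triggers the win screen when its box is overlapped.
; On BeginPlay, the timeline offsets the actor from the initial location cached in the Construction Script, without sweeping.
; A box overlap, with no check on the overlapping actor, creates the Win_Screen widget, focuses it in Game and UI input mode and pauses the game.
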(event OnComponentBeginOverlap(Box)
  (params (OverlappedComponent :type Primitive%20Component%20Object%20Reference) (OtherActor :type Actor%20Object%20Reference) (OtherComp :type Primitive%20Component%20Object%20Reference) (OtherBodyIndex :type Integer) (bFromSweep :type Boolean) (SweepResult :type Hit%20Result%20Structure%20%28by%20ref%29))
  (bind _returnvalue (UserInterface|CreateWidget "/Game/HUD/Win_Screen.Win_Screen_C")) ; declaring win screen
  (UserInterface|Viewport|AddtoViewport _returnvalue 0) ; adding screen widget to viewport
  (Input|SetInputModeGameandUI (Game|GetPlayerController 0) _returnvalue "DoNotLock" true) ; setting widget screen
  (Game|SetGamePaused true) ; pause game when widget is active
)

(event EventBeginPlay
  (bind _newtrack_2 (Timeline|Completion_Gate_Left_Right Play) ; timeline of platform movement
    (:Update
      (Transformation|SetActorLocation (+ (Variables|Default|GetInitial%20Location) _newtrack_2) false false) ; declaring new platform location
    )))

(fn ConstructionScript
  (bind _returnvalue (Transformation|GetActorLocation))
  (Transformation|SetActorLocation _returnvalue false false)
  (Variables|Default|SetInitial%20Location _returnvalue))