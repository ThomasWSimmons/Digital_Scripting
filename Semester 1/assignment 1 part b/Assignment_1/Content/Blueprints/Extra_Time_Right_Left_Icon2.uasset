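; Extra time pickup icon for a 2D side-scroller that moves, by its name right and left, and grants the player bonus seconds.
; The construction script stores the placed location, and a timeline started on BeginPlay offsets the actor from it each update.
; On overlap with the side-scroller character, it adds a fixed amount to that character's Timer and destroys itself.
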(event EventBeginPlay
  (bind _newtrack_0 (Timeline|Extra_Time_Icon Play) ; timeline of platform movement
    (:Update
      (Transformation|SetActorLocation (+ (Variables|Default|GetInitial%20Location) _newtrack_0) false false) ; declaring new platform location
    )))

(event Collision|EventActorBeginOverlap
  (params (OtherActor :type Actor%20Object%20Reference))
  (bind _as2dside_scroller_character (Utilities|Casting|CastTo2DSideScrollerCharacter OtherActor)) ; Declaring 2D player character
  (Variables|/Game/2DSideScrollerBP/Blueprints/2DSideScrollerCharacter.2DSideScrollerCharacter_C|SetTimer _as2dside_scroller_character (+ (Variables|/Game/2DSideScrollerBP/Blueprints/2DSideScrollerCharacter.2DSideScrollerCharacter_C|GetTimer _as2dside_scroller_character) 5.0)) ; set new timer to the HUD
  (Actor|DestroyActor) ; Destroy icon after colliding
)

(fn ConstructionScript
  (bind _returnvalue (Transformation|GetActorLocation))
  (Transformation|SetActorLocation _returnvalue false false)
  (Variables|Default|SetInitial%20Location _returnvalue))